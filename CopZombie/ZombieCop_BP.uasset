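; Zombie cop enemy character that roams to random navmesh points and chases the player on sight.
; PawnSensing reacts to first-person, VR and pickup-truck pawns, triggering a one-time scream and a run toward player 0.
; Projectile hits spawn blood and drain health until it is destroyed, while pickup overlaps play fall and stand-up animations before roaming resumes.
; Animations play directly on the mesh; car-hit physics, respawn and scoring logic are left unconnected.
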(event OnComponentHit(CapsuleComponent)
  (params (HitComponent :type Primitive%20Component%20Object%20Reference) (OtherActor :type Actor%20Object%20Reference) (OtherComp :type Primitive%20Component%20Object%20Reference) (NormalImpulse :type Vector :default "0, 0, 0") (Hit :type Hit%20Result%20Structure%20%28by%20ref%29))
  (Utilities|Casting|CastToFirstPersonProjectile OtherActor)
  (Effects|SpawnEmitterAttached "/Game/FXVillesBloodVFXPack/Particles/PS_Blood_Burst_Directional.PS_Blood_Burst_Directional" (Variables|Character|GetMesh) "None" "0, 0,150.000000")
  (Components|Animation|PlayAnimation (Variables|Character|GetMesh) "/Game/ZombieCharacters/Animations/Zombie_Death.Zombie_Death" false)
  (bind _output_get (Variables|Default|SetHealth (- (Variables|Default|GetHealth) 34)))
  (if (<= _output_get 0)
    (Class|Pawn|DetachfromControllerPendingDestroy)
    (Utilities|FlowControl|Delay 4.0)
    (Actor|DestroyActor)))

(event OnSeePawn(PawnSensing)
  (params (Pawn :type Pawn%20Object%20Reference))
  (Utilities|FlowControl|Sequence
    (:then_0
      ;[1 1 1] Zombie AI Chase or Idle
      (Utilities|Casting|CastToMotionControllerPawn Pawn)
      (bind _output_get (Variables|Default|SetSeen true))
      (if _output_get
        (Variables|Default|SetSeen false)
        (CallFunction|AiChase)
        (else
          (Utilities|FlowControl|RetriggerableDelay 1.0)
          (Variables|Default|SetSeen false)
          (CallFunction|MoveTorRandomLocation))))
    (:then_1
      (Utilities|Casting|CastToFirstPersonCharacter Pawn)
      (bind _output_get_2 (Variables|Default|SetSeen true))
      (if _output_get_2
        (Variables|Default|SetSeen false)
        (CallFunction|AiChase)
        (else
          (Utilities|FlowControl|RetriggerableDelay 2.5)
          (Variables|Default|SetSeen false)
          (CallFunction|MoveTorRandomLocation))))
    (:then_2
      (Utilities|Casting|CastToBP_Pickup Pawn)
      (bind _output_get_3 (Variables|Default|SetSeen true))
      (if _output_get_3
        (Variables|Default|SetSeen false)
        (CallFunction|AiChase)
        (else
          (Utilities|FlowControl|RetriggerableDelay 2.5)
          (Variables|Default|SetSeen false)
          (CallFunction|MoveTorRandomLocation))))))

(event OnComponentBeginOverlap(Mesh)
  (params (OverlappedComponent :type Primitive%20Component%20Object%20Reference) (OtherActor :type Actor%20Object%20Reference) (OtherComp :type Primitive%20Component%20Object%20Reference) (OtherBodyIndex :type Integer) (bFromSweep :type Boolean) (SweepResult :type Hit%20Result%20Structure%20%28by%20ref%29))
  (bind _mesh (Variables|Character|GetMesh))
  ;[1 1 1] Vehicle Zombie Collision Animation
  (Utilities|Casting|CastToBP_Pickup OtherActor)
  (Components|Animation|SetAnimationMode _mesh "AnimationBlueprint")
  (Components|Animation|PlayAnimation _mesh "/Game/ZombieCharacters/Animations/Zombie_Death.Zombie_Death" false)
  (Components|Animation|PlayAnimation (Variables|Character|GetMesh) "/Game/ZombieCharacters/Animations/Zombie_Stand_Up.Zombie_Stand_Up" false)
  (Pawn|Components|CharacterMovement|SetMovementMode (Variables|Character|GetCharacterMovement) "MOVE_Walking" 0)
  (CallFunction|MoveTorRandomLocation))

(event Custom|HitByCar
  (bind _capsulecomponent (Variables|Collision|GetCapsuleComponent))
  (Input|SetIgnoreMoveInput (Game|GetPlayerController 0) true)
  (Physics|SetSimulatePhysics _capsulecomponent true)
  (Collision|SetCollisionResponsetoChannel _capsulecomponent "ECC_Vehicle" "ECR_Block")
  (Utilities|FlowControl|Delay 0.5)
  (Class|PrimitiveComponent|PutRigidBodytoSleep (Variables|Collision|GetCapsuleComponent) (Class|SkinnedMeshComponent|GetBoneName (Variables|Character|GetMesh) 1))
  (Physics|SetSimulatePhysics (Variables|Collision|GetCapsuleComponent) false)
  (Utilities|FlowControl|Delay 0.2)
  (Input|ResetIgnoreMoveInput (Game|GetPlayerController 0))
  (Class|PrimitiveComponent|WakeRigidBody (Variables|Collision|GetCapsuleComponent) (Class|SkinnedMeshComponent|GetBoneName (Variables|Character|GetMesh) 1))
  (Transformation|SetActorRotation "0, 0, 0")
  (Class|SkeletalMeshComponent|SetAllBodiesBelowPhysicsBlendWeight (Variables|Character|GetMesh) (Class|SkinnedMeshComponent|GetBoneName (Variables|Character|GetMesh) 1) 0.0 false false)
  (Variables|Default|SetHitByCarTrue false))

(event Custom|MoveTorRandomLocation
  ;[1 1 1] AI Roam
  (AI|AIMoveTo self (.RandomLocation (Class|NavigationSystemV1|GetRandomPointinNavigableRadius (Transformation|GetActorLocation) 9e+02 0 0)) 0 15.0 false
    (:OnSuccess
      (Utilities|FlowControl|Delay 1.5)
      (Components|Animation|PlayAnimation (Variables|Character|GetMesh) "/Game/ZombieCharacters/Animations/Zombie_Walk.Zombie_Walk" true)
      (Variables|Default|SetSeen false))))

(event Custom|AiChase
  ;[1 1 1] Zombie AI Chase
  (Utilities|FlowControl|Sequence
    (:then_0
      (Utilities|FlowControl|DoOnce false
        (:Completed
          (CallFunction|AIScream))))
    (:then_1
      (AI|Navigation|SimpleMovetoActor (Pawn|GetController) (Game|Player|GetPlayerPawn 0))
      (Components|Animation|PlayAnimation (Variables|Character|GetMesh) "/Game/ZombieCharacters/Animations/Zombie_Running__3__Ch10_Anim_mixamo_com.Zombie_Running__3__Ch10_Anim_mixamo_com" true)
      (Utilities|FlowControl|Delay 1.0)
      (Variables|Default|SetSeen false))))

(event Custom|AI%20Scream
  ;[1 1 1] AI Scream
  (Components|Animation|PlayAnimation (Variables|Character|GetMesh) "/Game/ZombieCharacters/Animations/Zombie_Scream.Zombie_Scream" false)
  (Audio|PlaySoundatLocation "/Game/ZombieCharacters/Animations/Zombie_Long_Death-SoundBible_com-554299929.Zombie_Long_Death-SoundBible_com-554299929" "0, 0, 0" "0, 0, 0" 1.0 1.0 0.0 0 0 0))

(event EventBeginPlay
  (switch Utilities|FlowControl|Switch|SwitchonZombie1_Enum (Variables|Default|GetRoam)
    (:NewEnumerator1
      (CallFunction|MoveTorRandomLocation))))

(fn ConstructionScript)